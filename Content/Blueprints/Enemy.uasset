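; Enemy actor that moves along a spline path and reacts to damage with debug messages.
; Each tick it advances a travelled distance by speed and delta time, then sets its location to that point on the Path spline in world space.
; If no valid path is set, it prints an error and destroys itself.
; Taking damage only prints a message and the amount, with no health handling.
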(event `self.ReceiveTick`
  (params (DeltaSeconds :type "Float (single-precision)"))
  (`/Engine/EditorBlueprintResources/StandardMacros.IsValid` (`self.Path`)
    (:`Is Valid`
      (bind _output_get (set `self.Passed` (+ (* DeltaSeconds (`self.Speed`)) (`self.Passed`))))
      (`self.K2_SetActorLocation` (`SplineComponent.GetLocationAtDistanceAlongSpline` (`self.Path`) _output_get "World")))
    (:`Is Not Valid`
      (`KismetSystemLibrary.PrintString` "Spline not setup!" true true (struct :`R` 1.0 :`A` 1.0))
      (`self.K2_DestroyActor`))))

(event `self.ReceiveAnyDamage`
  (params (Damage :type "Float (single-precision)") (DamageType :type "DamageType Object Reference") (InstigatedBy :type "Controller Object Reference") (DamageCauser :type "Actor Object Reference"))
  (`KismetSystemLibrary.PrintString` "Ouch!")
  (`KismetSystemLibrary.PrintString` (`KismetStringLibrary.Conv_DoubleToString` Damage)))

(fn `UserConstructionScript`)