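; EnemyPath is an actor whose spline gives a path from its own location to a target, by default the BP_Core.
; All logic runs in the Construction Script, which auto-assigns Target when exactly one BP_Core exists and otherwise prints a red request for manual setup.
; With a valid Target, it seeds an empty spline with two world-space points, leaving any existing points untouched.
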(fn `UserConstructionScript`
  (`/Engine/EditorBlueprintResources/StandardMacros.IsValid` (`self.Target`)
    (:`Is Valid`
      (if (== (`SplineComponent.GetNumberOfSplinePoints` (`self.Path`)) 0) :!label _label
        (`SplineComponent.SetSplinePoints` (`self.Path`) (`|MakeArray` (`SceneComponent.K2_GetComponentLocation` (`self.Path`)) (`self.K2_GetActorLocation` (`self.Target`))) "World" true)))
    (:`Is Not Valid`
      (bind _outactors (`GameplayStatics.GetAllActorsOfClass` "/Game/Blueprints/BP_Core.BP_Core_C"))
      (if (== (`KismetArrayLibrary.Array_Length` _outactors) 1)
        (set `self.Target` (`|GetArrayItem` _outactors))
        (goto _label)
        (else
          (`KismetSystemLibrary.PrintString` "Can't setup target automatically, setup it manually, please" true true (struct :`R` 1.0 :`A` 1.0)))))))