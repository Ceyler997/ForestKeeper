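; Wave manager that runs the game's sequence of enemy waves from BeginPlay, with a delay before each one.
; Each wave maps path holders to enemy counts, and repeated timed stages spawn one enemy on every path with count remaining.
; Destroy callbacks track live enemies; when none remain it resets the stage counter and starts the next wave, or prints a win message after the last.
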(event `self.ReceiveBeginPlay`
  (`self.Start Wave`))

(event `Start Stage`
  (bind _is_finished (`self.Spawn Stage` (`|GetArrayItem` (`self.Waves`) (`self.Next Wave`))))
  (if (not _is_finished)
    (`KismetSystemLibrary.Delay` (`self.Enemy Spawn Delay`))
    (`self.Start Stage`)))

(event `Start Wave`
  (`KismetSystemLibrary.PrintString` "Delay before wave")
  (`KismetSystemLibrary.Delay` (`self.Wave Delay`))
  (`KismetSystemLibrary.PrintString` "Wave started")
  (`self.Start Stage`))

(fn `On Enemy Destroyed`
  (params (Enemy :type "Actor Object Reference"))
  (`KismetSystemLibrary.PrintString` "Enemy killed")
  (bind _result (`/Engine/EditorBlueprintResources/StandardMacros.DecrementInt` (`self.Current Enemies`))
    (:`  `
      (if (<= _result 0)
        (`KismetSystemLibrary.PrintString` "Wave killed")
        (bind _result_2 (`/Engine/EditorBlueprintResources/StandardMacros.IncrementInt` (`self.Next Wave`))
          (:`  `
            (set `self.Stages` 0)
            (if (>= _result_2 (`KismetArrayLibrary.Array_Length` (`self.Waves`)))
              (`KismetSystemLibrary.PrintString` "Win!" true true (struct :`G` 1.0 :`A` 1.0))
              (else
                (`self.Start Wave`)))))))))

(fn `Spawn Stage`
  (params (Wave :type "/Game/Blueprints/Wave Structure"))
  (returns (`Is Finished` :type Boolean))
  (locals (`Wave Map` :type "Map of /Game/Blueprints/EnemyPath Object Reference to Integer") (`Max Diff` :type Integer))
  (bind _max_diff (`local.Max Diff`))
  (bind _enemy_scale (`self.Enemy Scale`))
  (`KismetSystemLibrary.PrintString` "Stage started")
  (bind _output_get (set `local.Wave Map` (`.Wavelines_7_4986A0664DBFADA5E0FCDDB13487FB87` (break `/Game/Blueprints/Wave` Wave))))
  (bind _keys (`BlueprintMapLibrary.Map_Keys` _output_get))
  (for _array_element _keys
    (bind _returnvalue (- (`BlueprintMapLibrary.Map_Find` (`local.Wave Map`) _array_element) (`self.Stages`)))
    (set `local.Max Diff` (`KismetMathLibrary.Max` _returnvalue (`local.Max Diff`)))
    (if (> _returnvalue 0)
      (bind _returnvalue_2 (`|SpawnActorFromClass` "/Game/Blueprints/Enemy.Enemy_C" (`KismetMathLibrary.MakeTransform` (0.0 0.0 0.0) (struct) (`KismetMathLibrary.MakeVector` _enemy_scale _enemy_scale _enemy_scale)) "Undefined" "OverrideRootScale" null (`/Game/Blueprints/EnemyPath.Path` _array_element) null))
      (`/Engine/EditorBlueprintResources/StandardMacros.IsValid` _returnvalue_2
        (:`Is Valid`
          (`/Engine/EditorBlueprintResources/StandardMacros.IncrementInt` (`self.Current Enemies`)
            (:`  `
              (add `self.OnDestroyed` _returnvalue_2 (`|CreateDelegate` :!event `On Enemy Destroyed`))
              (`KismetSystemLibrary.PrintString` "Enemy Spawned")))))))
  (`/Engine/EditorBlueprintResources/StandardMacros.IncrementInt` (`self.Stages`)
    (:`  `
      (`KismetSystemLibrary.PrintString` "Stage finished")
      (`KismetSystemLibrary.PrintString` (`KismetStringLibrary.Conv_IntToString` _max_diff))
      (return (<= _max_diff 1)))))

(fn `UserConstructionScript`)