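; BP_Core is the base core the player defends, losing health whenever an Enemy overlaps its capsule.
; Each overlapping enemy subtracts its own core damage value from the health and is then destroyed.
; A dynamic material instance created at BeginPlay dims the mesh's emissive strength in proportion to remaining health.
; When health runs out, it prints a failure message and quits the game after a short delay.
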(event `self.ReceiveBeginPlay`
  (`|ExecutionSequence`
    (:`then_0`
      (bind _returnvalue (`PrimitiveComponent.CreateDynamicMaterialInstance` (`self.StaticMeshComponent`) 0 "/Game/Materials/MI_Core.MI_Core" "None"))
      (set `self.Material` _returnvalue))
    (:`then_1`
      (set `self.Current Health` (`self.Start Health`))
      (`self.Update Core Emissive`))))

(event `self.Capsule.OnComponentBeginOverlap`
  (params (OverlappedComponent :type "PrimitiveComponent Object Reference") (OtherActor :type "Actor Object Reference") (OtherComp :type "PrimitiveComponent Object Reference") (OtherBodyIndex :type Integer) (bFromSweep :type Boolean) (SweepResult :type "HitResult Structure (by ref)"))
  (bind _asenemy (cast `/Game/Blueprints/Enemy` OtherActor))
  (`|ExecutionSequence`
    (:`then_0`
      (set `self.Current Health` (- (`self.Current Health`) (`/Game/Blueprints/Enemy.DamageToCore` _asenemy)))
      (`self.K2_DestroyActor` _asenemy))
    (:`then_1`
      (`self.Update Core Emissive`))
    (:`then_2`
      (if (<= (`self.Current Health`) 0.0)
        (`KismetSystemLibrary.PrintString` "You've failed the level" true true (struct :`R` 1.0 :`A` 1.0))
        (`KismetSystemLibrary.Delay` 2.0)
        (`KismetSystemLibrary.QuitGame` null "Quit")))))

(fn `Update Core Emissive`
  (`MaterialInstanceDynamic.SetScalarParameterValue` (`self.Material`) "Emissive Strength" (* (`self.Start Emissive Value`) (/ (`self.Current Health`) (`self.Start Health`)))))

(fn `UserConstructionScript`)