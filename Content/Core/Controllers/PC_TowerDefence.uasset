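; Player controller for the tower defence game, turning mouse and key input into tower commands and spectator camera control.
; Clicks trace under the cursor to select and follow a tower, target an enemy or move the tower, while mode keys switch tower modes, all through an injected TowersController.
; Each tick, screen-edge cursor scrolling blends with axis input to move the P_Spectator pawn; axis input also stops following.
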(event `self.ReceiveBeginPlay`
  (`WidgetBlueprintLibrary.SetInputMode_GameOnly` self)
  (set `self.bShowMouseCursor` true)
  (bind _asp_spectator (cast `/Game/Core/Actors/P_Spectator` (`self.K2_GetPawn`)))
  (set `self.Spectator Pawn` _asp_spectator))

(event `self.ReceiveTick`
  (params (DeltaSeconds :type "Float (single-precision)"))
  (`self.Update Camera` DeltaSeconds))

(event `Key|LeftMouseButton`
  (params (Key :type "Key Structure"))
  (bind (_hitresult _returnvalue) (`self.GetHitResultUnderCursorByChannel` "TraceTypeQuery1" false))
  (bind (_bblockinghit _binitialoverlap _time _distance _location _impactpoint _normal _impactnormal _physmat _hitactor) (`GameplayStatics.BreakHitResult` _hitresult))
  ;[1 1 1] Left click
  (:`Pressed`
    (if _returnvalue
      (`|ExecutionSequence`
        (:`then_0`
          ;;[1 1 1] Handle if clicked on tower
          (bind _asp_tower (cast `/Game/Core/Actors/P_Tower` _hitactor))
          (`/Game/Core/Controllers/AIC_Tower.Select Tower` (`self.Towers Controller`) _asp_tower)
          (`/Game/Core/Actors/P_Spectator.Start Following Actor` (`self.Spectator Pawn`) _asp_tower))
        (:`then_1`
          ;;[1 1 1] Handle if clicked in enemy
          (bind _asp_enemy (cast `/Game/Core/Actors/P_Enemy` _hitactor))
          (`/Game/Core/Controllers/AIC_Tower.Select Tower Target` (`self.Towers Controller`) _asp_enemy))))))

(event `Key|RightMouseButton`
  (params (Key :type "Key Structure"))
  (bind (_hitresult _returnvalue) (`self.GetHitResultUnderCursorByChannel` "TraceTypeQuery3"))
  ;[1 1 1] Right click
  (:`Pressed`
    (if _returnvalue
      (`/Game/Core/Controllers/AIC_Tower.Move Tower to Location` (`self.Towers Controller`) (`.Location` (`GameplayStatics.BreakHitResult` _hitresult))))))

(event `InputAction|Mode 1`
  (params (Key :type "Key Structure"))
  ;[1 1 1] Modes switching
  (:`Pressed`
    (`/Game/Core/Controllers/AIC_Tower.Switch Tower Mode` (`self.Towers Controller`) "NewEnumerator0")))

(event `InputAction|Exit`
  (params (Key :type "Key Structure"))
  ;[1 1 1] Exit
  (:`Pressed`
    (bind _asgm_tower_defence (cast `/Game/Core/GM_TowerDefence` (`GameplayStatics.GetGameMode`))
      (:`then`
        (`/Game/Core/GM_TowerDefence.Exit` _asgm_tower_defence))
      (:`CastFailed`
        (`KismetSystemLibrary.QuitGame` null "Quit")))))

(event `InputAction|Mode 2`
  (params (Key :type "Key Structure"))
  ;[1 1 1] Modes switching
  (:`Pressed`
    (`/Game/Core/Controllers/AIC_Tower.Switch Tower Mode` (`self.Towers Controller`) "NewEnumerator1")))

(event `InputAction|Mode 3`
  (params (Key :type "Key Structure"))
  ;[1 1 1] Modes switching
  (:`Pressed`
    (`/Game/Core/Controllers/AIC_Tower.Switch Tower Mode` (`self.Towers Controller`) "NewEnumerator2")))

(event `InputAxis|Camera Up`
  (params (AxisValue :type "Float (single-precision)"))
  ;[1 1 1] Camera axis
  (if (not (`KismetMathLibrary.NearlyEqual_FloatFloat` AxisValue))
    (`/Game/Core/Actors/P_Spectator.Stop Following` (`self.Spectator Pawn`) :!label _label)))

(event `InputAxis|Camera Right`
  (params (AxisValue :type "Float (single-precision)"))
  ;[1 1 1] Camera axis
  (if (not (`KismetMathLibrary.NearlyEqual_FloatFloat` AxisValue))
    (goto _label)))

(event `InputAxis|Camera Zoom`
  (params (AxisValue :type "Float (single-precision)"))
  ;[1 1 1] Camera axis
  (`/Game/Core/Actors/P_Spectator.Zoom Camera` (`self.Spectator Pawn`) AxisValue))

(fn `Get Camera Axis Movement`
  (params (`Camera Axis Value` :type "Float (double-precision)") (threshold :type "Float (double-precision)"))
  (returns (`Camera Movement` :type "Float (double-precision)"))
  (bind _returnvalue (`KismetMathLibrary.FClamp` `Camera Axis Value`))
  (bind _returnvalue_2 (<= _returnvalue 0.5))
  (bind _returnvalue_3 (- 1.0 (`KismetMathLibrary.FClamp` (/ (select `bool` _returnvalue_2 :`false` (- 1.0 _returnvalue) :`true` _returnvalue) (`local.threshold`)))))
  (return (select `bool` _returnvalue_2 :`false` (* _returnvalue_3 -1.0) :`true` _returnvalue_3)))

(fn `Get Camera Move Vector`
  (params (`Mouse Viewport location` :type "Vector2D Structure"))
  (returns (`Camera Movement Vector` :type "Vector2D Structure"))
  (return (`KismetMathLibrary.MakeVector2D` (`KismetMathLibrary.FClamp` (+ (`self.Get Camera Axis Movement` `Mouse Viewport location_Y` (`self.Vertical threshold`)) (`self.GetInputAxisValue`)) -1.0) (`KismetMathLibrary.FClamp` (+ (* (`self.Get Camera Axis Movement` `Mouse Viewport location_X` (`self.Horizontal threshold`)) -1.0) (`self.GetInputAxisValue`)) -1.0))))

(fn `Set Towers Controller`
  (params (Controller :type "/Game/Core/Controllers/AIC_Tower Object Reference"))
  (set `self.Towers Controller` Controller))

(fn `Update Camera`
  (params (`Delta Seconds` :type "Float (double-precision)"))
  (`/Engine/EditorBlueprintResources/StandardMacros.IsValid` (`self.Spectator Pawn`)
    (:`Is Valid`
      (bind _returnvalue (`WidgetLayoutLibrary.GetMousePositionOnViewport`))
      (`/Game/Core/Actors/P_Spectator.Move Camera In Direction` (`self.Spectator Pawn`) (`self.Get Camera Move Vector` (/ (* _returnvalue (`WidgetLayoutLibrary.GetViewportScale`)) (`WidgetLayoutLibrary.GetViewportSize`)))))))

(fn `UserConstructionScript`)