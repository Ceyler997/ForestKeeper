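; Tower defence player controller that shows the mouse cursor, views through a child-actor camera and quits the game on the Exit input.
; Each tick it edge-scrolls the camera by moving the spring arm in world space, scaled by camera speed and delta time.
; The DPI-corrected, normalised mouse position becomes a signed per-axis strength, ramping linearly within threshold bands at the screen edges.
; Screen axes are swapped onto world axes, with horizontal negated.
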(event `self.ReceiveBeginPlay`
  (`self.SetViewTargetWithBlend` (`ChildActorComponent.ChildActor` (`self.Camera Actor`)))
  (set `self.bShowMouseCursor` true))

(event `self.ReceiveTick`
  (params (DeltaSeconds :type "Float (single-precision)"))
  (`self.Update Camera` DeltaSeconds))

(event `InputAction|Exit`
  (params (Key :type "Key Structure"))
  ;[1 1 1] Exit
  (:`Pressed`
    (`KismetSystemLibrary.QuitGame` null "Quit")))

(fn `Get Camera Axis Movement`
  (params (`Camera Axis Value` :type "Float (double-precision)") (threshold :type "Float (double-precision)"))
  (returns (`Camera Movement` :type "Float (double-precision)"))
  (bind _returnvalue (`KismetMathLibrary.FClamp` `Camera Axis Value`))
  (bind _returnvalue_2 (<= _returnvalue 0.5))
  (bind _returnvalue_3 (- 1.0 (`KismetMathLibrary.FClamp` (/ (select `bool` _returnvalue_2 :`false` (- 1.0 _returnvalue) :`true` _returnvalue) (`local.threshold`)))))
  (return (select `bool` _returnvalue_2 :`false` (* _returnvalue_3 -1.0) :`true` _returnvalue_3)))

(fn `Get Camera Move Vector`
  (params (`Mouse Viewport location` :type "Vector2D Structure"))
  (returns (`Camera Movement Vector` :type "Vector2D Structure"))
  (return (`KismetMathLibrary.MakeVector2D` (* (`self.Get Camera Axis Movement` `Mouse Viewport location_X` (`self.Horizontal threshold`)) -1.0) (`self.Get Camera Axis Movement` `Mouse Viewport location_Y` (`self.Vertical threshold`)))))

(fn `Update Camera`
  (params (`Delta Seconds` :type "Float (double-precision)"))
  (bind _returnvalue (`WidgetLayoutLibrary.GetMousePositionOnViewport`))
  (bind (_returnvalue_x _returnvalue_y) (`KismetMathLibrary.BreakVector2D` (* (`self.Get Camera Move Vector` (/ (* _returnvalue (`WidgetLayoutLibrary.GetViewportScale`)) (`WidgetLayoutLibrary.GetViewportSize`))) (* (`self.Camera Speed`) (`local.Delta Seconds`)))))
  (`SceneComponent.K2_AddWorldOffset` (`self.SpringArm`) (`KismetMathLibrary.MakeVector` _returnvalue_y _returnvalue_x) false false))

(fn `UserConstructionScript`)