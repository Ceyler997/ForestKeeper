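; Tower defence game mode that runs the wave sequence and decides win or loss.
; On BeginPlay it finds the single Core and single WaveManager actors in the level, printing an error if the count differs, and binds to their events.
; Each finished wave starts the next after a delay.
; Core death loses, finishing all waves with the Core alive wins, and either outcome prints a message and quits.
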(event `On Core Death`
  ;[1 1 1] Lose event (core death)
  (`self.K2_DestroyActor` (`self.Core`))
  (`KismetSystemLibrary.PrintString` "You lost" true true (struct :`R` 1.0 :`A` 1.0))
  (`KismetSystemLibrary.Delay` 2.0)
  (`KismetSystemLibrary.QuitGame` null "Quit"))

(event `self.ReceiveBeginPlay`
  (bind _wave_manager (`self.Wave Manager`))
  ;[1 1 1] Setup core
  (bind _core__nullable_ (`self.Get Core`))
  (bind _output_get (set `self.Core` _core__nullable_))
  (`/Engine/EditorBlueprintResources/StandardMacros.IsValid` _output_get
    (:`Is Valid`
      (`|ExecutionSequence`
        (:`then_0`
          ;[1 1 1] Lose event (core death)
          (add `/Game/Core/Actors/A_Core.On Death` (`self.Core`) (delegate `On Core Death`)))
        (:`then_1`
          ;[1 1 1] Setup wave manger
          (bind _wave_manager_2 (`self.Get Wave Manager`))
          (bind _output_get_2 (set `self.Wave Manager` _wave_manager_2))
          (`/Engine/EditorBlueprintResources/StandardMacros.IsValid` _output_get_2
            (:`Is Valid`
              (add `/Game/Core/Actors/A_WaveManager.On Wave Finished` _wave_manager (delegate `Wave Finished`))
              (add `/Game/Core/Actors/A_WaveManager.On All Waves Finished` _wave_manager (delegate `Waves finished`))
              ;[1 1 1] Start wave
              (`/Game/Core/Actors/A_WaveManager.Start Wave` (`self.Wave Manager`) 0))))))))

(event `Wave Finished`
  ;[1 1 1] Wave Finished event
  (`/Engine/EditorBlueprintResources/StandardMacros.IncrementInt` (`self.Current Wave Number`)
    (:`  `
      (`KismetSystemLibrary.Delay` (`self.Delay Between Waves`))
      (`/Game/Core/Actors/A_WaveManager.Start Wave` (`self.Wave Manager`) (`self.Current Wave Number`)))))

(event `Waves finished`
  (bind _core (`self.Core`))
  ;[1 1 1] Win event (end of waves)
  (`/Engine/EditorBlueprintResources/StandardMacros.IsValid` _core
    (:`Is Valid`
      (if (> (`/Game/Core/Actors/A_Core.Get Health` _core) 0.0)
        (`KismetSystemLibrary.PrintString` "You win" true true (struct :`G` 1.0 :`A` 1.0))
        (`KismetSystemLibrary.Delay` 2.0)
        (`KismetSystemLibrary.QuitGame` null "Quit")))))

(fn `Get Core`
  (returns (`Core (Nullable)` :type "/Game/Core/Actors/A_Core Object Reference"))
  (bind _outactors (`GameplayStatics.GetAllActorsOfClass` "/Game/Core/Actors/A_Core.A_Core_C"))
  (bind _returnvalue (`KismetArrayLibrary.Array_Length` _outactors))
  (if (== _returnvalue 1)
    (return (`|GetArrayItem` _outactors))
    (else
      (`KismetSystemLibrary.PrintString` (`KismetStringLibrary.Concat_StrStr` "There is " (`KismetStringLibrary.Conv_IntToString` _returnvalue) " cores, can't setup the game mode") true true (struct :`R` 1.0 :`A` 1.0))
      (return null))))

(fn `Get Wave Manager`
  (returns (`Wave Manager` :type "/Game/Core/Actors/A_WaveManager Object Reference"))
  (bind _outactors (`GameplayStatics.GetAllActorsOfClass` "/Game/Core/Actors/A_WaveManager.A_WaveManager_C"))
  (bind _returnvalue (`KismetArrayLibrary.Array_Length` _outactors))
  (if (== _returnvalue 1)
    (return (`|GetArrayItem` _outactors))
    (else
      (`KismetSystemLibrary.PrintString` (`KismetStringLibrary.Concat_StrStr` "There is " (`KismetStringLibrary.Conv_IntToString` _returnvalue) " wave managers, can't setup the game mode") true true (struct :`R` 1.0 :`A` 1.0))
      (return null))))

(fn `UserConstructionScript`)